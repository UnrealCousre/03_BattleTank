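; Player-controllable tank Blueprint that wires its components together and routes input for driving, camera aiming and firing.
; On BeginPlay it registers the barrel and turret components and initialises TankMovement with both tracks.
; Forward and turn input feed TankMovement as movement intents, while separate throttle axes drive each track directly.
; Aim axes rotate an azimuth gimbal for yaw and the spring arm for pitch, and the Fire action calls Fire.
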(event `self.ReceiveBeginPlay`
  (`self.SetBarrelComponent` (`self.TankBarrel`))
  (`self.SetTurretComponent` (`self.TankTurret`))
  (`TankMovementComponent.Initialise` (`self.TankMovement`) (`self.LeftTrack`) (`self.RIghtTrack`)))

(event `InputAxis|TurnRight`
  (params (AxisValue :type "Float (single-precision)"))
  (`TankMovementComponent.IntendTurnRight` (`self.TankMovement`) AxisValue))

(event `InputAxis|AimAzimuth`
  (params (AxisValue :type "Float (single-precision)"))
  (`SceneComponent.K2_AddLocalRotation` (`self.Azimuth Gimbal`) (`KismetMathLibrary.MakeRotator` 0.0 0.0 (* AxisValue 5.0)) false false))

(event `InputAxis|MoveForward`
  (params (AxisValue :type "Float (single-precision)"))
  (`TankMovementComponent.IntendMoveForward` (`self.TankMovement`) AxisValue))

(event `InputAxis|AimAltitude`
  (params (AxisValue :type "Float (single-precision)"))
  (`SceneComponent.K2_AddLocalRotation` (`self.SpringARm`) (`KismetMathLibrary.MakeRotator` 0.0 (* AxisValue 5.0)) false false))

(event `InputAxis|LeftTrackThrottle`
  (params (AxisValue :type "Float (single-precision)"))
  (`TrackComponent.SetThrottle` (`self.LeftTrack`) AxisValue))

(event `InputAction|Fire`
  (params (Key :type "Key Structure"))
  (:`Pressed`
    (`self.Fire`)))

(event `InputAxis|RightTrackThrottle`
  (params (AxisValue :type "Float (single-precision)"))
  (`TrackComponent.SetThrottle` (`self.RIghtTrack`) AxisValue))

(fn `UserConstructionScript`)